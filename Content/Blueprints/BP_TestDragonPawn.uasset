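; BP_TestDragonPawn is a test dragon pawn for trying out form setup, camera orientation and attack input.
; On BeginPlay it switches its FormComponent to the Base form, then after a short delay prints the follow camera's rotation minus the capsule's, labelled "Rel Loc" despite being rotation.
; The base and charged attack input actions only print their names as placeholders.
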(event `self.ReceiveBeginPlay`
  (bind (_returnvalue_roll _returnvalue_pitch _returnvalue_yaw) (`KismetMathLibrary.BreakRotator` (`SceneComponent.K2_GetComponentRotation` (`self.CapsuleComponent`))))
  (bind (_returnvalue_roll_2 _returnvalue_pitch_2 _returnvalue_yaw_2) (`KismetMathLibrary.BreakRotator` (`SceneComponent.K2_GetComponentRotation` (`self.FollowCamera`))))
  (`DragonFormComponent.SwitchForm` (`self.FormComponent`) (struct :`TagName` "Form.Base"))
  (`KismetSystemLibrary.Delay` 2.0)
  (`KismetSystemLibrary.PrintString` (`KismetStringLibrary.Concat_StrStr` "Rel Loc = " (`KismetStringLibrary.Conv_RotatorToString` (`KismetMathLibrary.MakeRotator` (- _returnvalue_roll_2 _returnvalue_roll) (- _returnvalue_pitch_2 _returnvalue_pitch) (- _returnvalue_yaw_2 _returnvalue_yaw)))) true true (struct :`G` 0.66 :`B` 1.0 :`A` 1.0) 10.0))

(event `EnhancedInput|/Game/Variant_Combat/Input/Actions/IA_BaseAttack`
  (params (ActionValue :type Boolean) (ElapsedSeconds :type "Float (double-precision)") (TriggeredSeconds :type "Float (double-precision)") (InputAction :type "InputAction Object Reference" :default "/Game/Variant_Combat/Input/Actions/IA_BaseAttack.IA_BaseAttack"))
  (:`Triggered`
    (`KismetSystemLibrary.PrintString` "BaseAttack")))

(event `EnhancedInput|/Game/Variant_Combat/Input/Actions/IA_ChargedAttack`
  (params (ActionValue :type Boolean) (ElapsedSeconds :type "Float (double-precision)") (TriggeredSeconds :type "Float (double-precision)") (InputAction :type "InputAction Object Reference" :default "/Game/Variant_Combat/Input/Actions/IA_ChargedAttack.IA_ChargedAttack"))
  (:`Triggered`
    (`KismetSystemLibrary.PrintString` "ChargedAttack")))

(fn `UserConstructionScript`)